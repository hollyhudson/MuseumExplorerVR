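; BP_Painting is a museum exhibit actor with an artifact receptacle that reports which artifacts rest on it.
; On BeginPlay it inserts its painting name as the first actor tag.
; GetReceptacleContents rebuilds and returns a unique list of BP_Artifact actors currently overlapping the receptacle.
; The begin and end overlap events are empty, and the logic for flagging artifacts as overlapping is disconnected.
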(event OnComponentBeginOverlap(ArtifactReceptacle)
  (params (OverlappedComponent :type Primitive%20Component%20Object%20Reference) (OtherActor :type Actor%20Object%20Reference) (OtherComp :type Primitive%20Component%20Object%20Reference) (OtherBodyIndex :type Integer) (bFromSweep :type Boolean) (SweepResult :type Hit%20Result%20Structure%20%28by%20ref%29)))

(event OnComponentEndOverlap(ArtifactReceptacle)
  (params (OverlappedComponent :type Primitive%20Component%20Object%20Reference) (OtherActor :type Actor%20Object%20Reference) (OtherComp :type Primitive%20Component%20Object%20Reference) (OtherBodyIndex :type Integer)))

(event EventBeginPlay
  ;[1 1 1] Add tag for painting name
  (Utilities|Array|Insert (Variables|Actor|GetTags) (Variables|Default|Getpainting_name)))

(fn ConstructionScript)

(fn GetReceptacleContents
  (Utilities|Array|Clear (Variables|Default|Getreceptacle_contents))
  (for _array_element (Collision|GetOverlappingActors (Variables|Default|GetArtifactReceptacle) "/Game/MuseumExplorer/Blueprints/BP_Artifact.BP_Artifact_C" :!class /Script/Engine.PrimitiveComponent)
    (bind _asbp_artifact (Utilities|Casting|CastToBP_Artifact _array_element))
    (Utilities|Array|AddUnique (Variables|Default|Getreceptacle_contents) _asbp_artifact))
  (return (Variables|Default|Getreceptacle_contents)))