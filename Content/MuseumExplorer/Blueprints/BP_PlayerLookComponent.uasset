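; Player look component meant to detect what the player looks at and message that actor, though all its logic is unwired and its events are empty.
; The disconnected graphs take the owner's camera as Eye and sphere-trace forward on Visibility.
; A new hit within that actor's reported maximum distance becomes LookatTarget and receives LookAtMessage.
; Otherwise the target clears, and an out-of-range hit also calls HideHUDMsg, intended to hide the ExplorerHUD message.
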(event Custom|HideHUDMsg)

(event EventBeginPlay
  ;[1 1 1] Initialize Eye on Camera
)

(event EventTick
  (params (DeltaSeconds :type Float%20%28single-precision%29))
  ;[1 1 1] What is the player looking at?
)