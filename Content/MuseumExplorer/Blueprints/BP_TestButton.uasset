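; Museum puzzle button that, on Use or overlap, checks whether the paintings' receptacles hold the correct items.
; It finds paintings by tags matching PaintingDataTable row names and requires each receptacle to hold exactly one item with a matching MatchId.
; A win changes the material and plays sound and explosion; a loss buzzes and flashes red through a timeline-driven dynamic material.
; Look-at highlighting and HUD message logic are present but disconnected.
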(event OnComponentBeginOverlap(Button)
  (params (OverlappedComponent :type Primitive%20Component%20Object%20Reference) (OtherActor :type Actor%20Object%20Reference) (OtherComp :type Primitive%20Component%20Object%20Reference) (OtherBodyIndex :type Integer) (bFromSweep :type Boolean) (SweepResult :type Hit%20Result%20Structure%20%28by%20ref%29))
  (CallFunction|Use))

(event EventLookat
  ;[1 1 1] Light up the button if we're looking at it
)

(event EventUse
  (bind _button (Variables|Default|GetButton))
  ;[1 1 1] Button press effects
  (Components|MoveComponentTo _button "0.0,0.0,2600" "0, 0,0.000000" true true 0.2 false)
  (Components|MoveComponentTo _button "0, 0,2700.000000" "0, 0,0.000000" true true 0.2 false)
  (Utilities|Array|Clear (Variables|Default|Getmatches))
  (Variables|Default|Setwon true)
  (bind _outrownames (DataTable|GetDataTableRowNames "/Game/MuseumExplorer/Data/PaintingDataTable.PaintingDataTable"))
  (for _array_element _outrownames
    (bind _outactors (Actor|GetAllActorswithTag _array_element))
    (for _array_element_2 _outactors
      (bind _asbp_painting (Utilities|Casting|CastToBP_Painting _array_element_2))
      (bind _contents (Default|GetReceptacleContents _asbp_painting))
      (if (== (Utilities|Array|Length _contents) 1)
        (Utilities|Array|Add (Variables|Default|Getmatches) (Utilities|Enum|Equal(Enum) (Variables|/Game/MuseumExplorer/Blueprints/BP_Painting.BP_Painting_C|Getmatch_id _asbp_painting) (Variables|/Game/MuseumExplorer/Blueprints/BP_Artifact.BP_Artifact_C|Getmatch_id (Utilities|Array|Get(acopy) _contents))))
        (else
          (Utilities|Array|Add (Variables|Default|Getmatches) (== (Utilities|Array|Length _contents) 1)))))
    (for _array_element_3 (Variables|Default|Getmatches)
      (if (not _array_element_3)
        (Variables|Default|Setwon false))))
  (if (Variables|Default|Getwon)
    ;[1 1 1] Win
    (Rendering|Material|SetMaterial (Variables|Default|GetButton) 0 "/Game/MuseumExplorer/Assets/Materials/M_ButtonFocused.M_ButtonFocused")
    (Audio|PlaySoundatLocation "/Game/MuseumExplorer/Assets/Audio/won.won" (Transformation|GetWorldLocation (Variables|Default|GetButton)))
    (Effects|SpawnEmitterAttached "/Game/MuseumExplorer/Particle_Systems/ExplodingBricks/WinningExplosion.WinningExplosion" (Variables|Default|GetButton) "None" "0, 0, 0" "0, 0, 0" "SnapToTarget")
    (else
      ;[1 1 1] Lose
      (Rendering|Material|SetMaterial (Variables|Default|GetButton) 0 (Variables|Default|Getredbuzzflash))
      (Audio|PlaySoundatLocation "/Game/MuseumExplorer/Assets/Audio/Rijks_buzz.Rijks_buzz" (Transformation|GetWorldLocation (Variables|Default|GetButton)))
      (bind _redness (Timeline|redbuzz Play)
        (:Update
          (Rendering|Material|SetScalarParameterValue (Variables|Default|Getredbuzzflash) "red_brightness" _redness :!class /Script/Engine.MaterialInstanceDynamic))))))

(event EventTick
  (params (DeltaSeconds :type Float%20%28single-precision%29))
  ;[1 1 1] Unlight the button if we're looking away
)

(event EventBeginPlay
  ;[1 1 1] Grab a reference to the ExplorerHUD
)

(fn ConstructionScript
  (bind _returnvalue (Rendering|Material|CreateDynamicMaterialInstance (Variables|Default|GetButton) 0 "/Game/MuseumExplorer/Assets/Materials/M_ButtonRedbuzz_Inst.M_ButtonRedbuzz_Inst" :!class /Script/Engine.PrimitiveComponent))
  (bind _output_get (Variables|Default|Setredbuzzflash _returnvalue))
  (Rendering|Material|SetScalarParameterValue _output_get "red_brightness" 0.0 :!class /Script/Engine.MaterialInstanceDynamic)
  (Rendering|Material|SetMaterial (Variables|Default|GetButton) 0 "/Game/MuseumExplorer/Assets/Materials/M_ButtonUnfocused.M_ButtonUnfocused"))

(fn GetMaxLookatDistance
  (return (Variables|Default|Getmax_look_distance)))